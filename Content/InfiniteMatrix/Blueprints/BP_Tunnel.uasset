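; BP_Tunnel is a tunnel segment with a spinning hole wall, used in a continuously spawned tunnel.
; Tick rolls the wall at RotateSpeed, and RandomizeWall picks one of four hole meshes with a random roll.
; When the player overlaps TriggerZone, TunnelSpawner spawns another tunnel and this one destroys itself.
; KillTunnelAll also destroys any health kit and enemy linked through BindExVars.
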(event `self.ReceiveTick`
  (params (DeltaSeconds :type "Float (single-precision)"))
  (`SceneComponent.K2_AddLocalRotation` (`self.WallMesh`) (`KismetMathLibrary.MakeRotator` (* DeltaSeconds (`self.RotateSpeed`))) false false))

(event `self.TriggerZone.OnComponentBeginOverlap`
  (params (OverlappedComponent :type "PrimitiveComponent Object Reference") (OtherActor :type "Actor Object Reference") (OtherComp :type "PrimitiveComponent Object Reference") (OtherBodyIndex :type Integer) (bFromSweep :type Boolean) (SweepResult :type "HitResult Structure (by ref)"))
  (cast `/Game/InfiniteMatrix/Blueprints/BP_Player` OtherActor)
  (`/Game/InfiniteMatrix/Blueprints/BP_TunnelSpawner.SpawnTunnelAtSpawnPoint` (`self.TunnelSpawner`))
  (`self.KillTunnelAll`))

(fn `BindExVars`
  (params (AssHealthKit :type "/Game/InfiniteMatrix/Blueprints/HealthKit Object Reference") (AssEnemy :type "/Game/InfiniteMatrix/Blueprints/Enemy Object Reference"))
  (set `self.HealthKitRef` AssHealthKit)
  (set `self.EnemyRef` AssEnemy))

(fn `KillTunnelAll`
  (bind _enemyref (`self.EnemyRef`))
  (bind _healthkitref (`self.HealthKitRef`))
  (if (`KismetSystemLibrary.IsValid` _healthkitref)
    (`self.K2_DestroyActor` _healthkitref))
  (if (`KismetSystemLibrary.IsValid` _enemyref)
    (`self.K2_DestroyActor` _enemyref))
  (`self.K2_DestroyActor`))

(fn `RandomizeWall`
  (`StaticMeshComponent.SetStaticMesh` (`self.WallMesh`) (select `int` (`KismetMathLibrary.RandomIntegerInRange` 0 3) :`0` "/Game/InfiniteMatrix/Meshes/SM_Hole_01.SM_Hole_01" :`1` "/Game/InfiniteMatrix/Meshes/SM_Hole_02.SM_Hole_02" :`2` "/Game/InfiniteMatrix/Meshes/SM_Hole_03.SM_Hole_03" :`3` "/Game/InfiniteMatrix/Meshes/SM_Hole_04.SM_Hole_04" :!type "StaticMesh Object Reference"))
  (`SceneComponent.K2_AddLocalRotation` (`self.WallMesh`) (`KismetMathLibrary.MakeRotator` (`KismetMathLibrary.RandomFloatInRange` 0.0 360.0)) false false))

(fn `UserConstructionScript`)