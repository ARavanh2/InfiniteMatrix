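; Projectile actor that destroys enemies and awards score to a player.
; Each tick it sweeps along world X by frame-scaled MoveSpeed plus SpeedScoreMod, which is not delta-scaled.
; Sphere overlaps ignore "Trigger" components; "Enemy" hits destroy that actor and loop ManageScore on PlayerRef, and any non-trigger hit destroys the bullet.
; SetPlayerRef supplies the player reference and speed modifier.
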(event `self.Sphere.OnComponentBeginOverlap`
  (params (OverlappedComponent :type "PrimitiveComponent Object Reference") (OtherActor :type "Actor Object Reference") (OtherComp :type "PrimitiveComponent Object Reference") (OtherBodyIndex :type Integer) (bFromSweep :type Boolean) (SweepResult :type "HitResult Structure (by ref)"))
  (if (`ActorComponent.ComponentHasTag` OtherComp "Trigger")
    _
    (elif (`ActorComponent.ComponentHasTag` OtherComp "Enemy")
      (`self.K2_DestroyActor` OtherActor)
      (for _ (range 3)
        (`/Game/InfiniteMatrix/Blueprints/BP_Player.ManageScore` (`self.PlayerRef`))
        (`self.K2_DestroyActor` :!label _label))
      (else
        (goto _label)))))

(event `self.ReceiveTick`
  (params (DeltaSeconds :type "Float (single-precision)"))
  (`self.K2_AddActorWorldOffset` (`KismetMathLibrary.MakeVector` (+ (* DeltaSeconds (`self.MoveSpeed`)) (`self.SpeedScoreMod`))) true))

(fn `SetPlayerRef`
  (params (NewPlayerRef :type "/Game/InfiniteMatrix/Blueprints/BP_Player Object Reference") (NewSpeedMod :type "Float (double-precision)"))
  (set `self.PlayerRef` NewPlayerRef)
  (set `self.SpeedScoreMod` NewSpeedMod))

(fn `UserConstructionScript`)