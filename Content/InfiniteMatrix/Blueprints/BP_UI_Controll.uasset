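; BP_UI_Controll is a HUD controller Blueprint that owns and updates the health and score widgets.
; On BeginPlay it creates WBP_Health and WBP_Score, stores references to them and adds both to the viewport.
; Its UpdateScoreUI and UpdateHealthUI events forward new values to those widgets through SetScore and SetHealth.
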(event `UpdateScoreUI`
  (params (new_score :type "Float (double-precision)"))
  (`/Game/InfiniteMatrix/UI/WBP_Score.SetScore` (`self.WB_Score`) new_score))

(event `UpdateHealthUI`
  (params (CurrHealth :type "Float (double-precision)") (MaxHealth :type "Float (double-precision)"))
  (`/Game/InfiniteMatrix/UI/WBP_Health.SetHealth` (`self.WB_health`) CurrHealth MaxHealth))

(event `self.ReceiveBeginPlay`
  (bind _returnvalue (`|CreateWidget` "/Game/InfiniteMatrix/UI/WBP_Health.WBP_Health_C"))
  (bind _output_get (set `self.WB_health` _returnvalue))
  (`UserWidget.AddToViewport` _output_get 0)
  (bind _returnvalue_2 (`|CreateWidget` "/Game/InfiniteMatrix/UI/WBP_Score.WBP_Score_C"))
  (bind _output_get_2 (set `self.WB_Score` _returnvalue_2))
  (`UserWidget.AddToViewport` _output_get_2 0))

(fn `UserConstructionScript`)