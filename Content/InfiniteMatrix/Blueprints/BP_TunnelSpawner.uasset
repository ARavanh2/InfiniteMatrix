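; Spawner that builds a chain of BP_Tunnel segments, each attached at the previous segment's SpawnPoint.
; On BeginPlay it calls KillTunnelAll on existing tunnels, then seeds a few segments, starting at the player pawn if none is tracked.
; Each spawn randomly adds an offset HealthKit or Enemy, or both, randomizes the wall, and passes the pickups and a spawner reference to the tunnel.
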(event `self.ReceiveBeginPlay`
  (`self.SpawnInitialTunnels`))

(fn `SpawnInitialTunnels`
  (`|ExecutionSequence`
    (:`then_0`
      (bind _outactors (`GameplayStatics.GetAllActorsOfClass` "/Game/InfiniteMatrix/Blueprints/BP_Tunnel.BP_Tunnel_C"))
      (for _array_element _outactors
        (`/Game/InfiniteMatrix/Blueprints/BP_Tunnel.KillTunnelAll` _array_element)))
    (:`then_1`
      (for _ (range 3)
        (`/Engine/EditorBlueprintResources/StandardMacros.IsValid` (`self.NewestTunnel`)
          (:`Is Valid`
            (`self.SpawnTunnelAtSpawnPoint`))
          (:`Is Not Valid`
            (`self.SpawnTunnel` (`self.K2_GetActorLocation` (`GameplayStatics.GetPlayerPawn` 0)))))))))

(fn `SpawnTunnel`
  (params (`Spawn location` :type "Vector Structure"))
  (bind _returnvalue (`|SpawnActorFromClass` "/Game/InfiniteMatrix/Blueprints/BP_Tunnel.BP_Tunnel_C" (`KismetMathLibrary.MakeTransform` `Spawn location`) "Undefined" "MultiplyWithRoot" null null))
  (if (not (> 80 (`KismetMathLibrary.RandomInteger` 100)))
    (bind _returnvalue_2 (`|SpawnActorFromClass` "/Game/InfiniteMatrix/Blueprints/HealthKit.HealthKit_C" (`KismetMathLibrary.MakeTransform` (+ `Spawn location` (+ (`KismetMathLibrary.MakeVector` (`KismetMathLibrary.RandomFloatInRange` -600.0 400.0) (`KismetMathLibrary.RandomFloatInRange` -300.0 300.0) (`KismetMathLibrary.RandomFloatInRange` -300.0 300.0)) (1500.0 0.0 0.0)))) "Undefined" "MultiplyWithRoot" null null)))
  (if (not (> 60 (`KismetMathLibrary.RandomInteger` 100)))
    (bind _returnvalue_3 (`|SpawnActorFromClass` "/Game/InfiniteMatrix/Blueprints/Enemy.Enemy_C" (`KismetMathLibrary.MakeTransform` (+ `Spawn location` (+ (`KismetMathLibrary.MakeVector` (`KismetMathLibrary.RandomFloatInRange` -600.0 400.0) (`KismetMathLibrary.RandomFloatInRange` -300.0 300.0) (`KismetMathLibrary.RandomFloatInRange` -300.0 300.0)) (1600.0 0.0 0.0)))) "Undefined" "MultiplyWithRoot" null null)))
  (bind _output_get (set `self.NewestTunnel` _returnvalue))
  (set `/Game/InfiniteMatrix/Blueprints/BP_Tunnel.TunnelSpawner` self _output_get)
  (`/Game/InfiniteMatrix/Blueprints/BP_Tunnel.RandomizeWall` _output_get)
  (`/Game/InfiniteMatrix/Blueprints/BP_Tunnel.BindExVars` _output_get _returnvalue_2 _returnvalue_3))

(fn `SpawnTunnelAtSpawnPoint`
  (`self.SpawnTunnel` (`SceneComponent.K2_GetComponentLocation` (`/Game/InfiniteMatrix/Blueprints/BP_Tunnel.SpawnPoint` (`self.NewestTunnel`)))))

(fn `UserConstructionScript`)